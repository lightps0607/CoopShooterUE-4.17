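; BP_AdvancedAI is an AI-controlled enemy that leaves a random drop behind when it dies.
; On BeginPlay its AI controller runs the BT_AdvancedAI behavior tree.
; Tick polls the Died flag and, through a DoOnce, waits briefly, then spawns an explosive barrel or HP drop with even odds at its transform.
; It then destroys its attached actors, but not itself in this graph.
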(event `self.ReceiveBeginPlay`
  (`AIController.RunBehaviorTree` (`AIBlueprintHelperLibrary.GetAIController` self) "/Game/AdvancedAI/BT_AdvancedAI.BT_AdvancedAI"))

(event `self.ReceiveTick`
  (params (DeltaSeconds :type "Float (single-precision)"))
  ;[1 1 1] Spawns Random on death
  (if (`self.bDied`)
    (`/Engine/EditorBlueprintResources/StandardMacros.DoOnce` false
      (:`Completed`
        (`KismetSystemLibrary.Delay` 1.0)
        (`|SpawnActorFromClass` (select `int` (`KismetMathLibrary.RandomIntegerInRange` 0 3) :`0` "/Game/Challenges/ExplosiveBarrel/BP_ExplosiveBarrel.BP_ExplosiveBarrel_C" :`1` "/Game/Blueprints/Extras/BP_HPDrop.BP_HPDrop_C" :`2` "/Game/Blueprints/Extras/BP_HPDrop.BP_HPDrop_C" :`3` "/Game/Challenges/ExplosiveBarrel/BP_ExplosiveBarrel.BP_ExplosiveBarrel_C" :!type "Actor Class Reference") (`self.GetTransform`) "Undefined" "OverrideRootScale" null null)
        (for _array_element (`self.GetAttachedActors`)
          (`self.K2_DestroyActor` _array_element))))))

(fn `UserConstructionScript`)