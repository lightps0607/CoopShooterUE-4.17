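; BP_BlackHole is a destructible objective actor that also spawns backup enemy AI while alive.
; Damage depletes HP; at zero a one-shot check requires ObjectiveSystem objective 3, then advances to 4, plays an effect, shows WBP_GameOver and destroys the actor.
; A looping timer spawns small random batches of TrackerBot or AdvancedAI at random TargetPoints, as a fallback for failed wave spawns.
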(event `self.ReceiveAnyDamage`
  (params (Damage :type "Float (single-precision)") (DamageType :type "DamageType Object Reference") (InstigatedBy :type "Controller Object Reference") (DamageCauser :type "Actor Object Reference"))
  (bind _output_get (set `self.HP` (- (`self.HP`) Damage)))
  (if (<= _output_get 0.0)
    (`/Engine/EditorBlueprintResources/StandardMacros.DoOnce` false
      (:`Completed`
        (bind _outactors (`GameplayStatics.GetAllActorsOfClass` "/Game/Blueprints/Extras/ObjectiveSystem.ObjectiveSystem_C"))
        (bind _output (`|GetArrayItem` _outactors))
        (if (== (`/Game/Blueprints/Extras/ObjectiveSystem.CurrentObj` _output) 3)
          (`/Game/Blueprints/Extras/ObjectiveSystem.Change Objective` _output 4)
          (`GameplayStatics.SpawnEmitterAtLocation` "/Game/Powerups/Effects/P_gold_ore_lost.P_gold_ore_lost" (`self.K2_GetActorLocation`))
          (bind _returnvalue (`|CreateWidget` "/Game/Blueprints/Extras/WBP_GameOver.WBP_GameOver_C"))
          (`UserWidget.AddToViewport` _returnvalue 0)
          (`self.K2_DestroyActor`))))))

(event `self.ReceiveBeginPlay`
  (set `self.HP` (`self.DefaulHP`))
  ;[1 1 1] AI Spanw Backup In Case Wave Spawn Stucks or fails
  (`KismetSystemLibrary.K2_SetTimerDelegate` (delegate `CustomEvent_0`) 10.0 true))

(event `CustomEvent_0`
  ;[1 1 1] AI Spanw Backup In Case Wave Spawn Stucks or fails
  (for _ (range (+ (`KismetMathLibrary.RandomIntegerInRange` 0 2) 1))
    (bind _outactors (`GameplayStatics.GetAllActorsOfClass` "/Script/Engine.TargetPoint"))
    (`AIBlueprintHelperLibrary.SpawnAIFromClass` (select `bool` (`KismetMathLibrary.RandomBool`) :`false` "/Game/AdvancedAI/BP_AdvancedAI.BP_AdvancedAI_C" :`true` "/Game/TrackerBot/BP_TrackerBot.BP_TrackerBot_C" :!type "Pawn Class Reference") null (`self.K2_GetActorLocation` (`|GetArrayItem` _outactors (`KismetMathLibrary.RandomIntegerInRange` 0 (`KismetArrayLibrary.Array_LastIndex` _outactors)))))))

(fn `UserConstructionScript`)