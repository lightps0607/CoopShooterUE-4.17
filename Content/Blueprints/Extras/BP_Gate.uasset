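; BP_Gate is an objective-locked gate that the player pawn opens by overlapping it when ObjectiveSystem is on objective 2.
; Success advances to objective 3, spawns BP_BlackHole at BHSpawnLoc, sets a three-second lifespan and opens a Tick Gate that slides two cubes apart vertically each frame.
; Otherwise it prints a find-the-key message; the DoOnce is never reset, so only the first player overlap is evaluated.
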(event `self.ReceiveTick`
  (params (DeltaSeconds :type "Float (single-precision)"))
  (`/Engine/EditorBlueprintResources/StandardMacros.Gate` true :!label _label
    (:`Exit`
      (`SceneComponent.K2_AddWorldOffset` (`self.CubeDown`) (0.0 0.0 -10.0) false true)
      (`SceneComponent.K2_AddWorldOffset` (`self.CubeUp`) (0.0 0.0 10.0) false true))))

(event `self.ReceiveActorBeginOverlap`
  (params (OtherActor :type "Actor Object Reference"))
  (cast `/Game/Blueprints/PlayerPawn` OtherActor)
  (`/Engine/EditorBlueprintResources/StandardMacros.DoOnce` false
    (:`Completed`
      (bind _outactors (`GameplayStatics.GetAllActorsOfClass` "/Game/Blueprints/Extras/ObjectiveSystem.ObjectiveSystem_C"))
      (bind _output (`|GetArrayItem` _outactors))
      (if (== (`/Game/Blueprints/Extras/ObjectiveSystem.CurrentObj` _output) 2)
        (`/Game/Blueprints/Extras/ObjectiveSystem.Change Objective` _output 3)
        (`|SpawnActorFromClass` "/Game/Blueprints/Extras/BP_BlackHole.BP_BlackHole_C" (`self.GetTransform` (`self.BHSpawnLoc`)) "Undefined" "OverrideRootScale" null null)
        (`self.SetLifeSpan` 3.0)
        (goto _label :!via `Open`)
        (else
          (`KismetSystemLibrary.PrintString` "Find The Key FIrst!!!" true true (struct :`R` 1.0 :`B` 0.255102 :`A` 1.0)))))))

(fn `UserConstructionScript`)