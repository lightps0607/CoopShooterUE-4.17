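; Actor or component-style objective tracker that shows the current game objective on the HUD.
; On BeginPlay it creates the HUD widget, adds it to the viewport and activates the first objective.
; ChangeObjective stores the objective index and, if the widget is valid, pushes the matching title from the ObjTitle array to the HUD text.
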(event `self.ReceiveBeginPlay`
  (bind _returnvalue (`|CreateWidget` "/Game/Blueprints/Extras/HUD.HUD_C"))
  (bind _output_get (set `self.WB_HUD` _returnvalue))
  (`UserWidget.AddToViewport` _output_get 0)
  (`self.Change Objective` 0))

(event `Change Objective`
  (params (Id :type Integer))
  (bind _wb_hud (`self.WB_HUD`))
  (set `self.CurrentObj` Id)
  (`/Engine/EditorBlueprintResources/StandardMacros.IsValid` _wb_hud
    (:`Is Valid`
      (`/Game/Blueprints/Extras/HUD.Set ObjText` _wb_hud (`KismetTextLibrary.Conv_StringToText` (`|GetArrayItem` (`self.ObjTitle`) (`self.CurrentObj`)))))))

(fn `UserConstructionScript`)